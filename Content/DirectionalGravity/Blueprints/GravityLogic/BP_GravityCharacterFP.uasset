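; First-person player character for the directional-gravity game, adding dash, death, restart, pause and level-save handling on top of its parent.
; BeginPlay fades in audio, tints the world material collection by level name and removes already-saved collectables.
; Tick triggers death when ungrounded checks three seconds apart fail, outside "Start".
; Death pulls the capsule into a spawned DeathBP with post-process changes, then loads the level's "_Red" variant, or "Start" from "EndGame".
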(event `self.ReceiveBeginPlay`
  (bind _audio (`self.Audio`))
  (`|ExecutionSequence`
    (:`then_0`
      (bind _outactors (`GameplayStatics.GetAllActorsOfClass` "/Game/EasySave/easySaveObject.easySaveObject_C"))
      (set `self.Savegame` (`|GetArrayItem` _outactors))
      (bind _outactors_2 (`GameplayStatics.GetAllActorsOfClass` "/Game/Assets/LevelBuilder/PPActor.PPActor_C"))
      (set `self.PostProcess` (`|GetArrayItem` _outactors_2))
      (`AudioComponent.SetVolumeMultiplier` _audio 0.0)
      (bind (_direction _newtrack_0) (`Timeline|Timeline_0` :!via `PlayFromStart`)
        (:`Update`
          (`AudioComponent.SetVolumeMultiplier` _audio _newtrack_0)
          (`/Engine/EditorBlueprintResources/StandardMacros.DoOnce` false
            (:`Completed`
              (`WidgetBlueprintLibrary.SetInputMode_GameOnly` (`GameplayStatics.GetPlayerController` 0))
              (set `self.LevelComplete` true)
              (`KismetMaterialLibrary.SetScalarParameterValue` "/Game/Assets/WorldCollection.WorldCollection" "EdgeEffectToggle" 1.0)
              (bind _returnvalue (`GameplayStatics.GetCurrentLevelName` true))
              (if (`KismetStringLibrary.Contains` _returnvalue "Red")
                (`KismetMaterialLibrary.SetScalarParameterValue` "/Game/Assets/WorldCollection.WorldCollection" "R" 1.0)
                (`KismetMaterialLibrary.SetScalarParameterValue` "/Game/Assets/WorldCollection.WorldCollection" "G")
                (`KismetMaterialLibrary.SetScalarParameterValue` "/Game/Assets/WorldCollection.WorldCollection" "B")
                (else
                  (`KismetMaterialLibrary.SetScalarParameterValue` "/Game/Assets/WorldCollection.WorldCollection" "R")
                  (`KismetMaterialLibrary.SetScalarParameterValue` "/Game/Assets/WorldCollection.WorldCollection" "G" -0.163033)
                  (`KismetMaterialLibrary.SetScalarParameterValue` "/Game/Assets/WorldCollection.WorldCollection" "B" 1.0))))))))
    (:`then_1`
      (bind _returnvalue_2 (`GameplayStatics.GetCurrentLevelName` true))
      (bind _returnvalue_3 (`GameplayStatics.DoesSaveGameExist` (`KismetStringLibrary.Concat_StrStr` "Collectable" _returnvalue_2)))
      (if _returnvalue_3
        (bind _outactors_3 (`GameplayStatics.GetAllActorsOfClass` "/Game/Assets/Collecable.Collecable_C"))
        (`self.K2_DestroyActor` (`|GetArrayItem` _outactors_3))))))

(event `self.ReceiveTick`
  (params (DeltaSeconds :type "Float (single-precision)"))
  (bind _isonground (`self.IsOnGround`))
  (bind (_relativerotation_roll _relativerotation_pitch _relativerotation_yaw) (`KismetMathLibrary.BreakRotator` (`SceneComponent.RelativeRotation` (`self.CameraHolder`))))
  (`parent.ReceiveTick` DeltaSeconds)
  (`|ExecutionSequence`
    (:`then_0`
      (`KismetSystemLibrary.Delay` 0.2)
      (bind _returnvalue (`GameplayStatics.GetCurrentLevelName` true))
      (if (`KismetStringLibrary.EqualEqual_StrStr` _returnvalue "Start")
        _
        (elif (not _isonground)
          (`KismetSystemLibrary.Delay` 3.0)
          (if (not _isonground)
            (`self.DeathEvent`)))))
    (:`then_1`
      (`KismetSystemLibrary.Delay` 0.2)
      (`SceneComponent.K2_SetRelativeRotation` (`self.SpringArm`) (`KismetMathLibrary.MakeRotator` _relativerotation_roll _relativerotation_pitch _relativerotation_yaw) false false))))

(event `Teleporting`
  (bind (_direction _newtrack_0) (`Timeline|Timeline_1` :!via `PlayFromStart`)
    (:`Update`
      (set `CameraComponent.FieldOfView` _newtrack_0 (`self.Camera`)))))

(event `Key|H`
  (params (Key :type "Key Structure"))
  (:`Pressed`
    (bind _returnvalue (`GameplayStatics.GetCurrentLevelName` true))
    (if (`KismetStringLibrary.EqualEqual_StrStr` _returnvalue "EndGame")
      (bind _foundwidgets (`WidgetBlueprintLibrary.GetAllWidgetsOfClass` "/Game/UI/Credits.Credits_C"))
      (`/Game/UI/Credits.Animate` (`|GetArrayItem` _foundwidgets)))))

(event `DeathEvent`
  (bind _walkcollision (`self.WalkCollision`))
  (set `self.dead` true)
  (`/Engine/EditorBlueprintResources/StandardMacros.DoOnce` false
    (:`Completed`
      (bind _returnvalue (`|SpawnActorFromClass` "/Game/Assets/DeathActionBP/DeathBP.DeathBP_C" (`KismetMathLibrary.MakeTransform` (`SceneComponent.K2_GetComponentLocation` (`self.Arrow`))) "AlwaysSpawn" "OverrideRootScale" null null))
      (bind _output_get (set `self.DeathLocation` (`SceneComponent.K2_GetComponentLocation` _walkcollision)))
      (bind (_direction _newtrack_0) (`Timeline|Timeline_2`)
        (:`Update`
          (`SceneComponent.K2_SetWorldLocation` _walkcollision (`KismetMathLibrary.VLerp` _output_get (`SceneComponent.K2_GetComponentLocation` (`/Game/Assets/DeathActionBP/DeathBP.Sphere` _returnvalue)) _newtrack_0) false false)
          (`/Engine/EditorBlueprintResources/StandardMacros.DoOnce` false
            (:`Completed`
              (bind (_direction_2 _newtrack_0_2) (`Timeline|Timeline_3`)
                (:`Update`
                  (set `PostProcessComponent.Settings` (make `PostProcessSettings` :`VignetteIntensity` _newtrack_0_2) (`/Game/Assets/LevelBuilder/PPActor.PostProcess` (`self.PostProcess`))))))))
        (:`Finished`
          (bind _returnvalue_2 (`GameplayStatics.GetCurrentLevelName` true))
          (if (`KismetStringLibrary.EqualEqual_StrStr` _returnvalue_2 "EndGame")
            (`GameplayStatics.OpenLevel` "Start")
            (elif (`KismetStringLibrary.Contains` _returnvalue_2 "Red")
              (`GameplayStatics.OpenLevel` (`KismetStringLibrary.Conv_StringToName` _returnvalue_2) true _returnvalue_2)
              (else
                (`GameplayStatics.OpenLevel` (`KismetStringLibrary.Conv_StringToName` (`KismetStringLibrary.Concat_StrStr` _returnvalue_2 "_Red")))))))))))

(event `InputAction|Pause`
  (params (Key :type "Key Structure"))
  (:`Pressed`
    (bind _returnvalue (`|CreateWidget` "/Game/UI/PauseMenu.PauseMenu_C"))
    (`UserWidget.AddToViewport` _returnvalue 0)))

(event `InputAction|Restart`
  (params (Key :type "Key Structure"))
  (:`Pressed`
    (if (not (`self.dead`))
      (bind _returnvalue (`GameplayStatics.GetCurrentLevelName` true))
      (`GameplayStatics.OpenLevel` (`KismetStringLibrary.Conv_StringToName` _returnvalue)))))

(event `InputAction|Dash`
  (params (Key :type "Key Structure"))
  (bind _currentdashnumber (`self.CurrentDashNumber`))
  (:`Pressed`
    (if (not (`self.dead`))
      (`|ExecutionSequence`
        (:`then_0`
          (`/Engine/EditorBlueprintResources/StandardMacros.Gate` true :!label _label
            (:`Exit`
              (if (>= (`self.DashLimit`) _currentdashnumber)
                (bind _result (`/Engine/EditorBlueprintResources/StandardMacros.IncrementInt` _currentdashnumber)
                  (:`  `
                    (set `self.CurrentDashNumber` _result)
                    (`PrimitiveComponent.AddImpulse` (`self.WalkCollision`) (* (`KismetMathLibrary.Normal` (`SceneComponent.GetForwardVector` (`self.Camera`))) (`self.DashStrength`)) "None" true)))))))
        (:`then_1`
          (goto _label :!via `Open`))
        (:`then_2`
          (`KismetSystemLibrary.Delay` 0.3)
          (goto _label :!via `Close`))))))

(fn `SaveGameFunc`
  (params (LevelNumber :type Integer))
  (`/Game/EasySave/easySaveObject.EasySaveValue` :`self` (`self.Savegame`) :`keyName` (`self.SavedLevel`) :`keyType` "NewEnumerator2" :`keyValue` (`KismetTextLibrary.Conv_IntToText` LevelNumber)))

(fn `UserConstructionScript`
  (`parent.UserConstructionScript`))